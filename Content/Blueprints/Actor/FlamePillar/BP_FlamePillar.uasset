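; BP_FlamePillar is a flame pillar actor that flickers its FireLight by animating the light's intensity.
; On BeginPlay, ChooseTimeLine switches on a random integer to start one of two intensity timelines, each of which calls it again on finishing for an endless loop.
; Timeline values scale BaseFlameIntensity through SetFlameIntensity.
; RandomInteger(1) only yields 0, so the second timeline is never selected.
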(event `self.ReceiveBeginPlay`
  (`self.ChooseTimeLine`))

(event `Start FlameIntensity_1`
  (bind (_direction `_새_트랙_0`) (`Timeline|FlameIntensity_1` :!via `PlayFromStart`)
    (:`Update`
      (`self.SetFlameIntensity` `_새_트랙_0`))
    (:`Finished`
      (`self.ChooseTimeLine`))))

(event `Start FlameIntensity_2`
  (bind (_direction `_새_트랙_0`) (`Timeline|FlameIntensity_2` :!via `PlayFromStart`)
    (:`Update`
      (`self.SetFlameIntensity` `_새_트랙_0`))
    (:`Finished`
      (`self.ChooseTimeLine`))))

(fn `ChooseTimeLine`
  (switch `int` (`KismetMathLibrary.RandomInteger` 1)
    (:`Default`
      (`self.Start FlameIntensity_1` :!label _label))
    (:`0`
      (goto _label))
    (:`1`
      (`self.Start FlameIntensity_2`))))

(fn `SetFlameIntensity`
  (params (A :type "Float (double-precision)"))
  (`LightComponent.SetIntensity` (`self.FireLight`) (* A (`self.BaseFlameIntensity`))))

(fn `UserConstructionScript`)