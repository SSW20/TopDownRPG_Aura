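; Fade actor that fades its mesh in and out by temporarily swapping in dynamic fade materials.
; The construction script caches the original materials and creates dynamic instances from FadeDynamicInstances.
; Fadein applies those instances by slot index and plays a timeline driving their "Fade" parameter, restoring the originals upon finishing at 1.
; FadeOut only reverses the timeline, without reapplying the dynamic materials.
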(event `self.ReceiveBeginPlay`)

(event `/Game/Blueprints/Actor/FadeActor/BI_FadeInterface.FadeIn`
  (`self.SetMaterialsToDynamic`)
  (bind (_direction _fade) (`Timeline|Fade Timeline` :!label _label)
    (:`Update`
      (for _array_element (`self.DynamicInstances`)
        (`MaterialInstanceDynamic.SetScalarParameterValue` _array_element "Fade" _fade)))
    (:`Finished`
      (`self.TimelineFinished` _fade))))

(event `/Game/Blueprints/Actor/FadeActor/BI_FadeInterface.FadeOut`
  (goto _label :!via `Reverse`))

(fn `ResetToOriginalMaterials`
  (for (_array_element _array_index) (`self.OriginalMatarials`)
    (`PrimitiveComponent.SetMaterial` (`self.Mesh`) _array_index _array_element)))

(fn `SetMaterialsToDynamic`
  (for (_array_element _array_index) (`self.DynamicInstances`)
    (`PrimitiveComponent.SetMaterial` (`self.Mesh`) _array_index _array_element)))

(fn `TimelineFinished`
  (params (InputPin :type "Float (single-precision)"))
  (if (>= InputPin 1.0)
    (`self.ResetToOriginalMaterials`)
    (elif (<= InputPin 0.0)
      _)))

(fn `UserConstructionScript`
  (`KismetArrayLibrary.Array_Clear` (`self.DynamicInstances`))
  (set `self.OriginalMatarials` (`MeshComponent.GetMaterials` (`self.Mesh`)))
  (for _array_element (`self.FadeDynamicInstances`)
    (bind _returnvalue (`KismetMaterialLibrary.CreateDynamicMaterialInstance` _array_element))
    (`KismetArrayLibrary.Array_AddUnique` (`self.DynamicInstances`) _returnvalue)))