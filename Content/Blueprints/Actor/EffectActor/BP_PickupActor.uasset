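; Pickup actor, apparently a potion, that handles spawn, idle motion and consume feedback, with no pickup logic of its own.
; On BeginPlay it plays a spawn sound and a timeline that moves and scales it, with a one-shot impact sound near the landing height.
; Optional looks come from timelines for sine bobbing and yaw rotation, the latter only if location movement is enabled.
; Destruction plays the consume sound.
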(event `self.ReceiveBeginPlay`
  (`GameplayStatics.PlaySoundAtLocation` (`self.PotionSpawnSound`) (`self.K2_GetActorLocation`) (struct) 1.0 1.0 0.0 null null null null)
  (`self.SpawnEffect`)
  (if (`self.bMoveActorLocation`)
    (`self.UpdateLocation`)
    (if (`self.bMoveActorRotation`)
      (`self.UpdateRotation`))))

(event `UpdateLocation`
  (bind (_direction _sin) (`Timeline|SinLocation`)
    (:`Update`
      (`self.K2_SetActorRelativeLocation` (+ (`self.K2_GetActorLocation`) (`KismetMathLibrary.MakeVector` 0.0 0.0 (* _sin (`self.LocationScale`))))))))

(event `UpdateRotation`
  (bind (_direction _rot) (`Timeline|Rotation`)
    (:`Update`
      (`SceneComponent.K2_SetRelativeRotation` (`self.RootComponent`) (`KismetMathLibrary.MakeRotator` 0.0 0.0 _rot) false true))))

(event `SpawnEffect`
  (bind (_direction _locationz _scale) (`Timeline|Location`)
    (:`Update`
      (if (`KismetMathLibrary.NearlyEqual_FloatFloat` _locationz -0.2 0.1)
        (`/Engine/EditorBlueprintResources/StandardMacros.DoOnce` false
          (:`Completed`
            (bind _returnvalue (+ (`self.K2_GetActorLocation`) (`KismetMathLibrary.MakeVector` 0.0 0.0 (* _locationz 4.0))))
            (`GameplayStatics.PlaySoundAtLocation` (`self.GroundImpactSound`) _returnvalue (struct) 1.0 1.0 0.0 null null null null))))
      (`self.K2_SetActorRelativeLocation` _returnvalue)
      (`self.SetActorScale3D` (`KismetMathLibrary.MakeVector` _scale _scale _scale)))))

(event `self.ReceiveDestroyed`
  (`GameplayStatics.PlaySoundAtLocation` (`self.PotionConsumeSound`) (`self.K2_GetActorLocation`) (struct) 1.0 1.0 0.0 null null null null))

(fn `ActorSpawnLocactionForTime`
  (params (A :type "Float (double-precision)"))
  (bind _returnvalue (`self.K2_GetActorLocation`))
  (if (`KismetMathLibrary.NearlyEqual_FloatFloat` A -0.2 0.01)
    (`/Engine/EditorBlueprintResources/StandardMacros.DoOnce` false
      (:`Completed`
        (`GameplayStatics.PlaySoundAtLocation` (`self.GroundImpactSound`) _returnvalue (struct) 1.0 1.0 0.0 null null null null))))
  (`self.K2_SetActorRelativeLocation` (+ _returnvalue (`KismetMathLibrary.MakeVector` 0.0 0.0 (* A 4.0)))))

(fn `UserConstructionScript`)