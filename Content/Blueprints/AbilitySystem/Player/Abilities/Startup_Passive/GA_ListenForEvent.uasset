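; Passive player gameplay ability that turns incoming Attributes gameplay events into a Gameplay Effect on its owner.
; On activation it waits for events under the Attributes tag hierarchy, then builds an outgoing spec from EffectClass.
; ApplyGE sets a SetByCaller magnitude for every EventTags entry: the event magnitude for the exact match, zero for the rest.
; The spec is then applied to self, so one effect class serves every listed attribute tag.
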(event `self.K2_ActivateAbility`
  (bind _returnvalue (`self.GetAbilitySystemComponentFromActorInfo`))
  (bind (_asynctaskproxy _payload) (`AbilityTask_WaitGameplayEvent.WaitGameplayEvent` (struct :`TagName` "Attributes") null false false)
    (:`EventReceived`
      (bind (_eventtag _instigator _target _optionalobject _optionalobject2 _contexthandle _instigatortags _targettags _eventmagnitude) (break `GameplayEventData` _payload))
      (set `self.Event Tag` _eventtag)
      (set `self.Event Magnitude` _eventmagnitude)
      (set `self.Spec` (`AbilitySystemComponent.MakeOutgoingSpec` _returnvalue (`self.EffectClass`) 0.0 (`AbilitySystemComponent.MakeEffectContext` _returnvalue)))
      (for _array_element (`self.EventTags`)
        (if (`BlueprintGameplayTagLibrary.MatchesTag` (`self.Event Tag`) _array_element true)
          (`self.ApplyGE` _array_element (`self.Event Magnitude`) (`self.Spec`))
          (else
            (`self.ApplyGE` _array_element 0.0 (`self.Spec`)))))
      (`AbilitySystemComponent.BP_ApplyGameplayEffectSpecToSelf` (`self.GetAbilitySystemComponentFromActorInfo`) (`self.Spec`)))))

(fn `ApplyGE`
  (params (Tag :type "GameplayTag Structure") (Magnitude :type "Float (double-precision)") (Spec :type "GameplayEffectSpecHandle Structure"))
  (`AbilitySystemBlueprintLibrary.AssignTagSetByCallerMagnitude` Spec Tag Magnitude))