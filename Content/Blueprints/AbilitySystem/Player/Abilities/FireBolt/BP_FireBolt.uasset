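; BP_FireBolt is the player's Fire Bolt ability actor, handling the bolt's impact effects and removal.
; Each Tick compares the current location with the previous one and treats movement of 10 units or less as an impact, without using collision events or scaling by delta time.
; On impact it spawns the impact sound and a fire explosion Niagara system at its location, then destroys itself.
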(event `self.ReceiveTick`
  (params (DeltaSeconds :type "Float (single-precision)"))
  (set `self.LastLocation` (`self.CurrentLocation`))
  (bind _output_get (set `self.CurrentLocation` (`self.K2_GetActorLocation`)))
  (if (<= (`KismetMathLibrary.VSize` (- _output_get (`self.LastLocation`))) 10.0)
    (`GameplayStatics.SpawnSoundAtLocation` "/Game/Assets/Sounds/Abilities/FireBolt/sfx_FireBolt_Impact.sfx_FireBolt_Impact" (`self.CurrentLocation`) (struct) 1.0 1.0 0.0 null null)
    (`NiagaraFunctionLibrary.SpawnSystemAtLocation` "/Game/Assets/Effects/Projectiles/FireExplosion/NS_FireExplosion2.NS_FireExplosion2" (`self.CurrentLocation`))
    (`self.K2_DestroyActor`)))

(fn `UserConstructionScript`)