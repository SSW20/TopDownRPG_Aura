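; GA_FireBolt is the player's Fire Bolt gameplay ability, casting homing fire projectiles at the target under the mouse cursor.
; After committing, it reads cursor target data, turns the avatar toward the hit location via CombatInterface and plays the cast montage.
; The montage's Event.Montage.FireBolt gameplay event triggers SpawnProjectiles with a pitched launch homing on the hit actor, and the montage ending or being interrupted ends the ability.
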(event `self.K2_ActivateAbility`
  (bind _returnvalue (`self.K2_CommitAbility`))
  (if _returnvalue
    (bind (_asynctaskproxy _data) (`TargetDataUnderCursor.GetTargetDataUnderMouseCursor`)
      (:`ValidData`
        (bind (_bblockinghit _binitialoverlap _time _distance _location _impactpoint _normal _impactnormal _physmat _hitactor) (`GameplayStatics.BreakHitResult` (`AbilitySystemBlueprintLibrary.GetHitResultFromTargetData` _data)))
        (set `self.TargetLocation` _location)
        (set `self.Hit Actor` _hitactor)
        (bind _ascombat_interface (cast `CombatInterface` (`self.GetAvatarActorFromActorInfo`)))
        (`CombatInterface.SetFacingTarget` _ascombat_interface (`self.TargetLocation`))
        (`AbilityTask_PlayMontageAndWait.CreatePlayMontageAndWaitProxy` "None" "/Game/Assets/Characters/Aura/Animations/Abilities/AM_Cast_FireBolt.AM_Cast_FireBolt" 1.0 "None" false
          (:`then`
            (`AbilityTask_WaitGameplayEvent.WaitGameplayEvent` (struct :`TagName` "Event.Montage.FireBolt") null
              (:`EventReceived`
                (`self.SpawnProjectiles` (`self.TargetLocation`) true 45.0 (`self.Hit Actor`) true))))
          (:`OnCompleted`
            (`self.K2_EndAbility` :!label _label))
          (:`OnInterrupted`
            (goto _label))
          (:`OnCancelled`
            (goto _label)))))))