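; Fireball actor for the player's FireBlast ability that flies out, returns to its instigator and explodes.
; StartOutgoingTimeline runs server-side, using one timeline to lerp it forward and a second to home back to the instigator's current location.
; Within ExplodeDistance, it calls OnHit, applies radial damage through GAS DamageEffectParams to nearby live players except the owner, with per-target death and knockback impulses, then destroys itself.
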(event `self.StartOutgoingTimeline`
  (bind _returnvalue (`self.GetOwner`))
  (`/Engine/EditorBlueprintResources/ActorMacros.Switch Has Authority`
    (:`Authority`
      (`/Engine/EditorBlueprintResources/ActorMacros.Switch Has Authority`
        (:`Authority`
          (set `self.InitialLocation` (`self.K2_GetActorLocation`))
          (set `self.EndLocation` (+ (* (`self.GetActorForwardVector`) 400.0) (`self.InitialLocation`)))
          (bind (_direction _speed) (`Timeline|타임라인`)
            (:`Update`
              (`self.K2_SetActorLocation` (`KismetMathLibrary.VLerp` (`self.InitialLocation`) (`self.EndLocation`) _speed)))
            (:`Finished`
              (set `self.EndLocation` (`self.K2_GetActorLocation`))
              (bind (_direction_2 _speed_2) (`Timeline|타임라인_0`)
                (:`Update`
                  (`self.K2_SetActorLocation` (`KismetMathLibrary.VLerp` (`self.EndLocation`) (`self.K2_GetActorLocation` (`self.Instigator`)) _speed_2))
                  (if (`self.IsWithinExplodeDistance`)
                    (`self.OnHit`)
                    (bind _outoverlappingactors (`AuraAbilitySystemLibrary.GetLivePlayersWithInRadius` _returnvalue (`|MakeArray` _returnvalue) 200.0 (`self.K2_GetActorLocation`)))
                    (setmembers `DamageEffectParams` :`StructRef` (`self.ExplosionDamageParams`) :`bIsRadialDamage` true :`InnerRadialDamage` 50.0 :`OuterRadialDamage` 100.0 :`RadialOrigin` (`self.K2_GetActorLocation`))
                    (for _array_element _outoverlappingactors
                      (bind _structout (setmembers `DamageEffectParams` :`StructRef` (`self.ExplosionDamageParams`) :`TargetAbilitySystemComponent` (`AbilitySystemBlueprintLibrary.GetAbilitySystemComponent` _array_element) :`DeathImpulseVector` (`self.CalculateDeathImulseVector` _array_element) :`KnockbackImpulseVector` (`self.CalculateKnockBackImulseVector` _array_element)))
                      (`AuraAbilitySystemLibrary.ApplyDamageEffect` _structout))
                    (`self.K2_DestroyActor`)))))))))))

(fn `CalculateDeathImulseVector`
  (params (self2 :type "Actor Object Reference"))
  (returns (ReturnValue :type "Vector Structure"))
  (bind (_returnvalue_roll _returnvalue_pitch _returnvalue_yaw) (`KismetMathLibrary.BreakRotator` (`KismetMathLibrary.MakeRotFromX` (- (`self.K2_GetActorLocation` self2) (`self.K2_GetActorLocation`)))))
  (return (* (`KismetMathLibrary.GetForwardVector` (`KismetMathLibrary.MakeRotator` _returnvalue_roll 45.0 _returnvalue_yaw)) 15000.0)))

(fn `CalculateKnockBackImulseVector`
  (params (self2 :type "Actor Object Reference"))
  (returns (ReturnValue :type "Vector Structure"))
  (return (- (`self.K2_GetActorLocation` self2) (`self.K2_GetActorLocation`))))

(fn `IsWithinExplodeDistance`
  (returns (ReturnValue :type Boolean))
  (return (<= (`KismetMathLibrary.VSize` (- (`self.K2_GetActorLocation`) (`self.K2_GetActorLocation` (`self.Instigator`)))) (`self.ExplodeDistance`))))

(fn `UserConstructionScript`)