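; GA_MeleeAttack is a gameplay ability that performs a melee attack with a randomly chosen tagged montage from the avatar.
; While the montage plays, it waits for a gameplay event matching that montage's tag, then queries the avatar's combat socket location for that tag.
; It damages non-friendly live players within a small radius of that point, then ends; montage completion, interruption or cancellation also ends it.
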(event `self.K2_ActivateAbility`
  (bind _returnvalue (`self.GetAvatarActorFromActorInfo`))
  (bind _returnvalue_2 (message `CombatInterface.GetTaggedMontages` (`self.GetAvatarActorFromActorInfo`)))
  (bind _output_get (set `self.MontageAndTag` (`|GetArrayItem` _returnvalue_2 (`KismetMathLibrary.RandomIntegerInRange` 0 (- (`KismetArrayLibrary.Array_Length` _returnvalue_2) 1)))))
  (bind (_montage _montagetag) (break `TaggedMontage` _output_get))
  (`AbilityTask_PlayMontageAndWait.CreatePlayMontageAndWaitProxy` "None" _montage
    (:`then`
      (`AbilityTask_WaitGameplayEvent.WaitGameplayEvent` _montagetag null
        (:`EventReceived`
          (bind _returnvalue_3 (message `CombatInterface.GetCombatSocketLocation` _returnvalue _montagetag))
          (bind _outoverlappingactors (`AuraAbilitySystemLibrary.GetLivePlayersWithInRadius` _returnvalue (`|MakeArray` _returnvalue) 30.0 _returnvalue_3))
          (for _array_element _outoverlappingactors
            (bind _returnvalue_4 (`AuraAbilitySystemLibrary.IsFriend` (`self.GetAvatarActorFromActorInfo`) _array_element))
            (if (not _returnvalue_4)
              (`self.CauseDamage` _array_element)))
          (`self.K2_EndAbility`))))
    (:`OnCompleted`
      (`self.K2_EndAbility` :!label _label))
    (:`OnInterrupted`
      (goto _label))
    (:`OnCancelled`
      (goto _label))))