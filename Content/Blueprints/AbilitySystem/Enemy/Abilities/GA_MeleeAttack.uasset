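; GA_MeleeAttack is an enemy melee gameplay ability that turns the avatar toward its combat target and strikes.
; It plays a montage picked from the avatar's tagged montages and waits for that montage's attack-tag gameplay event.
; On the event, it sphere-checks live players around the tagged socket, damaging non-friends with possible knockback.
; A hit fires a MeleeImpact gameplay cue, and the ability ends after the event or montage end.
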(event `self.K2_ActivateAbility`
  (bind _returnvalue (`self.GetAvatarActorFromActorInfo`))
  (bind _returnvalue_2 (`self.GetAvatarActorFromActorInfo`))
  (bind (_montageandtag_montage _montageandtag_sockettag _montageandtag_attacktag) (break `TaggedMontage` (`self.MontageAndTag`)))
  (set `self.IsHit` false)
  (bind _returnvalue_3 (message `EnemyInterface.GetCombatTarget` _returnvalue_2))
  (bind _ascombat_interface (cast `CombatInterface` _returnvalue_2))
  (`CombatInterface.SetFacingTarget` _ascombat_interface (`Actor.K2_GetActorLocation` _returnvalue_3))
  (bind _returnvalue_4 (message `CombatInterface.GetTaggedMontages` (`self.GetAvatarActorFromActorInfo`)))
  (bind _output_get (set `self.MontageAndTag` (`self.GetTaggedMontageInArray` _returnvalue_4)))
  (bind (_montage _sockettag _attacktag) (break `TaggedMontage` _output_get))
  (`AbilityTask_PlayMontageAndWait.CreatePlayMontageAndWaitProxy` "None" _montage
    (:`then`
      (`AbilityTask_WaitGameplayEvent.WaitGameplayEvent` _attacktag null
        (:`EventReceived`
          (bind _returnvalue_5 (message `CombatInterface.GetCombatSocketLocation` _returnvalue _sockettag))
          (bind _output_get_2 (set `self.SocketLocation` _returnvalue_5))
          (bind _outoverlappingactors (`AuraAbilitySystemLibrary.GetLivePlayersWithInRadius` _returnvalue (`|MakeArray` _returnvalue) 30.0 _output_get_2))
          (for _array_element _outoverlappingactors
            (bind _returnvalue_6 (`AuraAbilitySystemLibrary.IsFriend` (`self.GetAvatarActorFromActorInfo`) _array_element))
            (if (not _returnvalue_6)
              (bind _returnvalue_7 (`self.DetermineKnockBack` _array_element (`self.MakeDamgeEffectParamsFromClassDefaults` _array_element)))
              (`AuraAbilitySystemLibrary.ApplyDamageEffect` _returnvalue_7)
              (set `self.IsHit` true)))
          (if (`self.IsHit`)
            (bind _returnvalue_8 (message `EnemyInterface.GetCombatTarget` (`self.GetAvatarActorFromActorInfo`)))
            (`self.K2_ExecuteGameplayCueWithParams` (struct :`TagName` "GameplayCue.MeleeImpact") (`AbilitySystemBlueprintLibrary.MakeGameplayCueParameters` 0.0 0.0 (struct) (struct) (struct) (`BlueprintGameplayTagLibrary.MakeGameplayTagContainerFromTag` _montageandtag_attacktag) (struct) (`self.SocketLocation`) (0.0 0.0 0.0) null (`self.GetAvatarActorFromActorInfo`) _returnvalue_8)))
          (`self.K2_EndAbility`))))
    (:`OnCompleted`
      (`self.K2_EndAbility` :!label _label))
    (:`OnInterrupted`
      (goto _label))
    (:`OnCancelled`
      (goto _label))))