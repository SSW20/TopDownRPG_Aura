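; GA_RangedAttack is an enemy gameplay ability that plays a ranged attack montage and fires a projectile at the combat target.
; On activation it faces the target through avatar messages, selects a tagged montage and plays it.
; The montage's attack tag gameplay event triggers the projectile spawn at the target's current location, then ends the ability.
; Montage completion, interruption or cancellation also ends it.
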(event `self.K2_ActivateAbility`
  (bind _returnvalue (`self.GetAvatarActorFromActorInfo`))
  (bind _returnvalue_2 (`self.GetAvatarActorFromActorInfo`))
  (bind _returnvalue_3 (message `EnemyInterface.GetCombatTarget` _returnvalue))
  (message `CombatInterface.SetFacingTarget` _returnvalue (`Actor.K2_GetActorLocation` _returnvalue_3))
  (bind _returnvalue_4 (message `CombatInterface.GetTaggedMontages` (`self.GetAvatarActorFromActorInfo`)))
  (bind _output_get (set `self.MontageAndTag` (`self.GetTaggedMontageInArray` _returnvalue_4)))
  (bind (_montage _sockettag _attacktag) (break `TaggedMontage` _output_get))
  (`AbilityTask_PlayMontageAndWait.CreatePlayMontageAndWaitProxy` "None" _montage 1.0 "None" false
    (:`then`
      (`AbilityTask_WaitGameplayEvent.WaitGameplayEvent` _attacktag null
        (:`EventReceived`
          (message `CombatInterface.GetCombatSocketLocation` _returnvalue_2 _sockettag)
          (bind _returnvalue_5 (message `EnemyInterface.GetCombatTarget` _returnvalue_2))
          (`self.SpawnProjectileInBluePrint` (`Actor.K2_GetActorLocation` _returnvalue_5))
          (`self.K2_EndAbility`))))
    (:`OnCompleted`
      (`self.K2_EndAbility` :!label _label))
    (:`OnInterrupted`
      (goto _label))
    (:`OnCancelled`
      (goto _label))))